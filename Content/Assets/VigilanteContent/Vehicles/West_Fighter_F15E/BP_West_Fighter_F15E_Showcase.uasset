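; Showcase Blueprint of the F-15E fighter that lets generic slider, twin-slider and checkbox inputs drive the aircraft's animated parts and visual states.
; Each input event forwards its value to setters for control surfaces, exhaust nozzles, lights, canopy, landing gear, hook, air brake, damage and afterburner.
; Left and right parts share one input, with the right aileron negated to deflect opposite the left.
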(event EventBeginPlay
  (|CallParentFunction) ; This node is disabled and will not be called.\nDrag off pins to build functionality.
)

(event Collision|EventActorBeginOverlap
  (params (OtherActor :type Actor%20Object%20Reference))
  (|CallParentFunction OtherActor) ; This node is disabled and will not be called.\nDrag off pins to build functionality.
)

(event EventSetSliderVariable6
  (params (NewValue :type Float%20%28double-precision%29))
  (CallFunction|SetCanopyOpen NewValue))

(event EventSetTwinSliderVariable1
  (params (bFirstSlider? :type Boolean) (NewFirstValue :type Float%20%28double-precision%29) (NewSecondValue :type Float%20%28double-precision%29))
  (CallFunction|SetHookAngle NewFirstValue)
  (CallFunction|SetAirBrake NewSecondValue))

(event EventSetCheckboxVariable0
  (params (NewState :type Boolean))
  (CallFunction|SetShowDamaged NewState))

(event EventSetCheckboxVariable1
  (params (NewState :type Boolean))
  (CallFunction|SetAfterburner NewState))

(event EventTick
  (params (DeltaSeconds :type Float%20%28single-precision%29))
  (|CallParentFunction DeltaSeconds) ; This node is disabled and will not be called.\nDrag off pins to build functionality.
)

(event EventSetSliderVariable0
  (params (NewValue :type Float%20%28double-precision%29))
  (CallFunction|SetRudder NewValue))

(event EventSetSliderVariable1
  (params (NewValue :type Float%20%28double-precision%29))
  (CallFunction|SetStabilizersL NewValue)
  (CallFunction|SetStabilizersR NewValue))

(event EventSetSliderVariable2
  (params (NewValue :type Float%20%28double-precision%29))
  (CallFunction|SetAileronL NewValue)
  (CallFunction|SetAileronR (* NewValue -1.0)))

(event EventSetSliderVariable3
  (params (NewValue :type Float%20%28double-precision%29))
  (CallFunction|SetFlapsL NewValue)
  (CallFunction|SetFlapsR NewValue))

(event EventSetSliderVariable4
  (params (NewValue :type Float%20%28double-precision%29))
  (CallFunction|SetExhaustNozzles NewValue))

(event EventSetSliderVariable5
  (params (NewValue :type Float%20%28double-precision%29))
  (CallFunction|SetLightsEmissivity NewValue))

(event EventSetTwinSliderVariable0
  (params (bFirstSlider? :type Boolean) (NewFirstValue :type Float%20%28double-precision%29) (NewSecondValue :type Float%20%28double-precision%29))
  (CallFunction|RetractFrontWheel NewFirstValue)
  (CallFunction|RetractRearLWheel NewSecondValue)
  (CallFunction|RetractRearRWheel NewSecondValue))

(fn ConstructionScript
  (|CallParentFunction))